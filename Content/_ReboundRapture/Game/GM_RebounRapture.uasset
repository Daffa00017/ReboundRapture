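; Game mode for Rebound Rapture that spawns the follow camera at the player and serves bullet trail and impact effects.
; BP_Effects actors are pooled through interface events, with a new one spawned when the pool has none valid.
; Each effect plays one of three random flipbook variants, cached by name.
; Uncached sets async-load from a data table, and a looping timer polls until all variants are valid before caching and playing.
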(event EventBeginPlay
  (bind _returnvalue (Game|SpawnActorfromClass "/Game/_ReboundRapture/Blueprint/Camera/BP_DownWellLiteCam.BP_DownWellLiteCam_C" (Math|Transform|MakeTransform (Transformation|GetActorLocation (Game|GetPlayerCharacter 0)) "0, 0, 0" "1.000000,1.000000,1.000000") "Undefined" "MultiplyWithRoot" 0 0))
  (bind _output_get (Variables|Default|SetCameraManager _returnvalue))
  (Class|CPPCameraManager|AdoptasViewTarget _output_get 0.25))

(event EventTick
  (params (DeltaSeconds :type Float%20%28single-precision%29)))

(event EventIGMSpawnFVX
  (params (PoolSize :type Integer))
  (for _index (range 0 PoolSize)
    (bind _returnvalue (Game|SpawnActorfromClass "/Game/_ReboundRapture/Blueprint/VFX/BP_Effects.BP_Effects_C" (Math|Transform|MakeTransform "0, 0, 0" "0, 0, 0" "1.000000,1.000000,1.000000") "Undefined" "MultiplyWithRoot" 0 self 0))
    (bind _output_get (Variables|Default|SetFVXRef _returnvalue))
    (Utilities|Array|Add (Variables|Default|GetFVXPool) _output_get)))

(event EventIGMPoolFVX
  (params (Reff :type Object%20Object%20Reference))
  (Utilities|Array|Add (Variables|Default|GetFVXPool) Reff))

(event EventIGMActivateTrailandBulletImpact
  (params (MuzzleLoc :type Vector :default "0, 0, 0") (ImpactLoc :type Vector :default "0, 0, 0") (AnimName :type Name :default "None"))
  (bind _fvxanimpool (Variables|Default|GetFVXAnimPool))
  (bind (_value _returnvalue) (Utilities|Map|Find _fvxanimpool AnimName))
  (if _returnvalue
    (CallFunction|ActivateFVX MuzzleLoc ImpactLoc _value)
    (else
      (|AsyncLoadVFX_2 MuzzleLoc ImpactLoc AnimName))))

(fn ConstructionScript)

(fn ActivateFVX
  (params (MuzzleLoc :type Vector) (FVXLoc :type Vector) (FlipbookAnim :type VFX%20Animation%20Resolved%20Structure))
  (bind (_animvar1 _animvar2 _animvar3) (Utilities|Struct|BreakVFXAnimationResolved FlipbookAnim))
  (bind _fvxpool (Variables|Default|GetFVXPool))
  (bind _output (Utilities|Array|Get(acopy) _fvxpool))
  (LocalVariables|SetAnimToPlay (Utilities|Select :Index (Math|Random|RandomIntegerinRange 0 2) :Option%200 _animvar1 :Option%201 _animvar2 :Option%202 _animvar3))
  (Utilities|IsValid _output
    (:Is%20Valid
      (Class|BPIActor|IActivateTrailandBulletImpact(Message) _output MuzzleLoc FVXLoc (LocalVariables|GetAnimToPlay))
      (Utilities|Array|RemoveItem (Variables|Default|GetFVXPool) _output))
    (:Is%20Not%20Valid
      (bind _returnvalue (Game|SpawnActorfromClass "/Game/_ReboundRapture/Blueprint/VFX/BP_Effects.BP_Effects_C" (Math|Transform|MakeTransform "0, 0, 0" "0, 0, 0" "1.000000,1.000000,1.000000") "Undefined" "MultiplyWithRoot" 0 self 0))
      (Class|BPIActor|IActivateTrailandBulletImpact(Message) _returnvalue MuzzleLoc FVXLoc (LocalVariables|GetAnimToPlay)))))

(event Custom|Timer_CheckAnimValid
  (bind _s_fvx (Variables|Default|Gets_Fvx))
  (if (Math|Boolean|ANDBoolean (Utilities|IsValid (Variables|Default|GetPf_VFXAnimVar3)) (Utilities|IsValid (Variables|Default|GetPf_VFXAnimVar1)) (Utilities|IsValid (Variables|Default|GetPf_VFXAnimVar2)))
    (Utilities|Map|Add (Variables|Default|GetFVXAnimPool) (Variables|Default|Getn_VFXAnimName) _s_fvx)
    (CallFunction|ActivateFVX (Variables|Default|Getv_MuzzleLoc) (Variables|Default|Getv_ImpactLoc) _s_fvx)
    (Utilities|Time|ClearandInvalidateTimerbyHandle (Variables|Default|GetTh_CheckAnim))
    (else
      (Development|PrintString "AnimStillAsyncLoad"))))