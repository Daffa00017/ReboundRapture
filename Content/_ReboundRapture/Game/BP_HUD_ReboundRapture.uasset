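; Rebound Rapture HUD Blueprint that relays gameplay UI events to the gameplay UI widget.
; It receives interface-style events for play, death, restart, score, health and ammo changes, including max values and ammo fills.
; Each event forwards its values unchanged as the matching message on the stored widget reference, with no logic of its own.
; This graph does not create or assign that reference.
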(event EventBeginPlay)

(event Collision|EventActorBeginOverlap
  (params (OtherActor :type Actor%20Object%20Reference)))

(event EventIUIonDeath
  (Class|BPIHUDandUI|IUIonDeath(Message) (Variables|Default|GetWB_GameplayUIReference)))

(event EventIUIRestart
  (Class|BPIHUDandUI|IUIRestart(Message) (Variables|Default|GetWB_GameplayUIReference)))

(event EventTick
  (params (DeltaSeconds :type Float%20%28single-precision%29)))

(event EventIUIonPlay
  (Class|BPIHUDandUI|IUIonPlay(Message) (Variables|Default|GetWB_GameplayUIReference)))

(event EventIUIBlponCurrentAmmoChange
  (params (CurrentAmmoIn :type Integer))
  (Class|BPIHUDandUI|IUIBlponCurrentAmmoChange(Message) (Variables|Default|GetWB_GameplayUIReference) CurrentAmmoIn))

(event EventIUIBlponMaxAmmoChange
  (params (MaxAmmoIn :type Integer))
  (Class|BPIHUDandUI|IUIBlponMaxAmmoChange(Message) (Variables|Default|GetWB_GameplayUIReference) MaxAmmoIn))

(event EventIUIBlponAmmoFill
  (params (CurrentAmmoIn :type Integer))
  (Class|BPIHUDandUI|IUIBlponAmmoFill(Message) (Variables|Default|GetWB_GameplayUIReference) CurrentAmmoIn))

(event EventIUIonMaxHealthChange
  (params (MaxHealthIn :type Float%20%28double-precision%29))
  (Class|BPIHUDandUI|IUIonMaxHealthChange(Message) (Variables|Default|GetWB_GameplayUIReference) MaxHealthIn))

(event EventIUIonHealthChange
  (params (CurrentHealthIn :type Float%20%28double-precision%29))
  (Class|BPIHUDandUI|IUIonHealthChange(Message) (Variables|Default|GetWB_GameplayUIReference) CurrentHealthIn))

(event EventIUIBlpUpdateScore
  (params (NewScoreIn :type Float%20%28double-precision%29))
  (Class|BPIHUDandUI|IUIBlpUpdateScore(Message) (Variables|Default|GetWB_GameplayUIReference) NewScoreIn))

(fn ConstructionScript)