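; BP_Blp_EnemiesFly is a flying enemy for the Bottomless Pit minigame, with pooled activation and deactivation events.
; It initializes its HitImpactComp on BeginPlay and triggers that component's damage flash whenever it takes any damage.
; The pool events only print debug messages with the actor's name, and the graph holds no movement or attack logic.
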(event EventBeginPlay
  (Default|InitHitImpactComponent (Variables|Default|GetHitImpact%20Comp)))

(event Collision|EventActorBeginOverlap
  (params (OtherActor :type Actor%20Object%20Reference)))

(event EventTick
  (params (DeltaSeconds :type Float%20%28single-precision%29)))

(event EventOnPooledActivated
  (Development|PrintString (Utilities|String|Append "Actor Activated : " (Utilities|GetDisplayName self)) true true "(R=0.000000,G=1.000000,B=0.029075,A=1.000000)"))

(event EventOnPooledDeactivated
  (Development|PrintString (Utilities|String|Append "Actor Deactivated : " (Utilities|GetDisplayName self)) true true "(R=1.000000,G=0.000000,B=0.024878,A=1.000000)"))

(event Game|Damage|EventAnyDamage
  (params (Damage :type Float%20%28single-precision%29) (DamageType :type Damage%20Type%20Object%20Reference) (InstigatedBy :type Controller%20Object%20Reference) (DamageCauser :type Actor%20Object%20Reference))
  (Default|StartDamagedFlash (Variables|Default|GetHitImpact%20Comp)))

(fn ConstructionScript)