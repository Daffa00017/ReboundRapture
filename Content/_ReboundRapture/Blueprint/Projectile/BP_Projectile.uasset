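; Pooled projectile Blueprint that takes its configuration by name from a data table and fires from a given start location.
; On activation it loads the flipbook config row asynchronously, caches it per name, then applies it and fires.
; A valid blocking hit triggers impact, deactivation and point damage.
; Deactivation sends the projectile to the game mode's pool through an interface message.
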(event Custom|OnDeactivated_Event
  (params (Projectile :type CPP%20Projectile%20Parent%20Object%20Reference))
  (Class|BPIGameMode|IGMPoolProjectile(Message) (Game|GetGameMode) self))

(event Custom|OnBlock_Event
  (params (Projectile :type CPP%20Projectile%20Parent%20Object%20Reference) (Hit :type Hit%20Result%20Structure%20%28by%20ref%29))
  (bind _hitactor (Collision|BreakHitResult Hit))
  (bind _self self)
  (Utilities|IsValid _hitactor
    (:Is%20Valid
      (Class|CPPProjectileParent|TriggerImpactandDeactivate Hit)
      (Game|Damage|ApplyPointDamage _hitactor 1.0 (Transformation|GetActorLocation _self) Hit 0 _self))))

(event EventBeginPlay
  (|bindEvent))

(event Collision|EventActorBeginOverlap
  (params (OtherActor :type Actor%20Object%20Reference)))

(event EventTick
  (params (DeltaSeconds :type Float%20%28single-precision%29)))

(event EventIActivateProjectile
  (params (ProjectileName :type Name :default "None") (StartLoc :type Vector :default "0, 0, 0"))
  (Variables|Default|Setv_CurrentStartLoc StartLoc)
  (Variables|Default|Setn_CurrentProjectileName ProjectileName)
  (if (.ReturnValue (Utilities|Map|Find (Variables|Default|GetS_SaveProjectileStat) (Variables|Default|Getn_CurrentProjectileName)))
    (Class|CPPProjectileParent|ApplyRuntimeConfig (.Value (Utilities|Map|Find (Variables|Default|GetS_SaveProjectileStat) (Variables|Default|Getn_CurrentProjectileName))))
    (Class|CPPProjectileParent|FirefromBP (Variables|Default|Getv_CurrentStartLoc))
    (else
      (bind _config (|LoadProjectileFlipbooksRowAsync (Variables|Default|GetDT_Projectile) (Variables|Default|Getn_CurrentProjectileName))
        (:OnCompleted
          (Utilities|Map|Add (Variables|Default|GetS_SaveProjectileStat) (Variables|Default|Getn_CurrentProjectileName) _config)
          (Class|CPPProjectileParent|ApplyRuntimeConfig _config)
          (Class|CPPProjectileParent|FirefromBP (Variables|Default|Getv_CurrentStartLoc)))))))

(fn ConstructionScript)