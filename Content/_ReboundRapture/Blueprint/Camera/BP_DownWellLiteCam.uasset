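; Orthographic follow camera for Rebound Rapture that tracks the player and reacts to first input, death and restart events.
; On first input, a timeline eases the follow lerp speed from a fast to a slower value.
; On death it focuses on the player and a timeline zooms in, then triggers the player's game-over sequence.
; Restart cancels focus and reverses that same timeline, restoring the fast follow speed once finished.
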(event Custom|SetCamPlay
  (bind _alpha (Timeline|LerpCamSpeed PlayFromStart)
    (:Update
      (Variables|Default|SetFollowLerpSpeed (Math|Float|Lerp 6e+01 6.0 _alpha)))))

(event Custom|OnRestartCameraLerp
  (bind _f_originalorthowidth (Variables|Default|Getf_OriginalOrthoWidth))
  (bind (_direction _alpha) (Timeline|LerpCamDead ReverseFromEnd)
    (:Update
      (Variables|Default|SetOrthoWidth (Math|Float|Lerp _f_originalorthowidth (- _f_originalorthowidth 7.5e+02) _alpha)))
    (:Finished
      (if (Utilities|Enum|Equal(Enum) _direction "Forward")
        (Class|BPIPlayer|IP1PlayGameOverSequence(Message) (Game|GetPlayerCharacter 0))
        (else
          (Variables|Default|SetFollowLerpSpeed 6e+01))))))

(event Custom|OnDeathCamera%20Lerp
  (bind _f_originalorthowidth (Variables|Default|Getf_OriginalOrthoWidth))
  (bind (_direction _alpha) (Timeline|LerpCamDead PlayFromStart)
    (:Update
      (Variables|Default|SetOrthoWidth (Math|Float|Lerp _f_originalorthowidth (- _f_originalorthowidth 7.5e+02) _alpha)))
    (:Finished
      (if (Utilities|Enum|Equal(Enum) _direction "Forward")
        (Class|BPIPlayer|IP1PlayGameOverSequence(Message) (Game|GetPlayerCharacter 0))
        (else
          (Variables|Default|SetFollowLerpSpeed 6e+01))))))

(event EventBeginPlay
  (Variables|Default|SetFollowTarget (Game|GetPlayerCharacter 0))
  (Variables|Default|SetFollowLerpSpeed 6e+01)
  (Variables|Default|Setf_OriginalOrthoWidth (Variables|Default|GetOrthoWidth)))

(event Collision|EventActorBeginOverlap
  (params (OtherActor :type Actor%20Object%20Reference)))

(event EventTick
  (params (DeltaSeconds :type Float%20%28single-precision%29)))

(event EventICamonFirstInput
  (CallFunction|SetCamPlay))

(event EventICamonDead
  (Class|CPPCameraManager|FocusonActor (Variables|Default|GetFollowTarget) 4e+01 true 0.0 0.0)
  (CallFunction|OnDeathCameraLerp))

(event EventICamonRestart
  (CallFunction|OnRestartCameraLerp)
  (Class|CPPCameraManager|CancelFocus))

(fn ConstructionScript)