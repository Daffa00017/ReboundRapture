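; BP_Gun is a gun with a Paper2D flipbook sprite that fires hitscan shots toward and past the cursor.
; On BeginPlay it snaps its muzzle to the flipbook's MuzzleSocket, and the IShoot event triggers the hitscan.
; On a hit, it messages the game mode through an interface to show a trail and bullet impact animation, passing the gun pivot's location as the trail start.
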(event EventBeginPlay
  (Transformation|AttachComponentToComponent (Variables|Default|GetMuzzle) (Variables|Default|GetGunFlipbook) "MuzzleSocket" "SnapToTarget" "SnapToTarget" "SnapToTarget" true))

(event EventIShoot
  (params (ArmDirection :type Vector :default "0, 0, 0"))
  (Class|CPPGun|CoreHitscanfromMuzzlePastCursor))

(event EventShootonHit
  (params (ShootResult :type Hit%20Result%20Structure))
  (Class|BPIGameMode|IGMActivateTrailandBulletImpact(Message) (Game|GetGameMode) (Transformation|GetWorldLocation (Variables|Default|GetGunPivot)) (.Location (Collision|BreakHitResult ShootResult)) "BulletImpact"))

(fn ConstructionScript)