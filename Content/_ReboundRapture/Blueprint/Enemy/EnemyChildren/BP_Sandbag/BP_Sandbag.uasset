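; BP_Sandbag is a sandbag enemy, a child Blueprint that reacts visually whenever it takes damage.
; On BeginPlay it runs the parent logic, then initializes its ACHitImpact1 hit-impact component.
; AnyDamage plays the Sb_Hurt sequence as an animation override on BodyAnim, then starts the component's damage flash.
; It adds no other behavior, as Tick and overlap are disabled and construction only calls the parent.
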(event EventBeginPlay
  (|CallParentFunction)
  (Default|PawnInitHitImpactComponent (Variables|Default|GetAC_HitImpact1)))

(event Collision|EventActorBeginOverlap
  (params (OtherActor :type Actor%20Object%20Reference))
  (|CallParentFunction OtherActor) ; This node is disabled and will not be called.\nDrag off pins to build functionality.
)

(event EventTick
  (params (DeltaSeconds :type Float%20%28single-precision%29)))

(event Game|Damage|EventAnyDamage
  (params (Damage :type Float%20%28single-precision%29) (DamageType :type Damage%20Type%20Object%20Reference) (InstigatedBy :type Controller%20Object%20Reference) (DamageCauser :type Actor%20Object%20Reference))
  (|PlayAnimationOverridewithCallbacks (Variables|/Script/PaperZD.PaperZDAnimationComponent|GetAnimInstance (Variables|Default|GetBodyAnim)) "/Game/_ReboundRapture/Blueprint/Enemy/Animation/AnimSequences/Sb_Hurt.Sb_Hurt" "DefaultSlot" 1.0 0.0
    (:then
      (Default|StartDamagedFlash (Variables|Default|GetAC_HitImpact1)))))

(fn ConstructionScript
  (|CallParentFunction))